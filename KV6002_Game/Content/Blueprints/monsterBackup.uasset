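; Paper2D monster actor that takes damage as one of four types (skeleton, mushroom, goblin, eye), with a health bar widget.
; doDamage decrements Health and plays that type's hit flipbook; death plays its death flipbook, then recycles the actor as a different random type with restored health.
; Tick polls PlayerLives, and at zero grants an achievement, opens GameOver, stops audio and only then checks Health for death.
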(event Custom|checkPlayerLives
  ;[1 1 1] Player Lives
  (if (<= (Variables|Default|GetplayerLives) 0)
    (Class|AchievementSubSystem|AddAchievementProgress (Subsystems|GetAchievementSubSystem) "Ach3" 1.0)
    (Game|OpenLevel(byName) "GameOver")))

(event Custom|randomMonster
  ;[1 1 1] Makes a different random monster
  (bind _output_get (Variables|Default|SetnewMonsterType (Math|Random|RandomIntegerinRange 0 3)))
  (if (== _output_get (Variables|Default|GetmonsterType))
    (CallFunction|RandomMonster)
    (else
      (Variables|Default|SetmonsterType (Variables|Default|GetnewMonsterType)))))

(event Custom|death
  ;[1 1 1] Skeleton death
  (if (== (Variables|Default|GetmonsterType) 0)
    (Sprite|SetFlipbook (Variables|Default|GetRenderComponent) "/Game/Monsters/Monsters_Creatures_Fantasy/Skeleton/skeletonDeath.skeletonDeath")
    (Components|Timeline|SetLooping (Variables|Default|GetRenderComponent) false)
    (Utilities|FlowControl|Delay (- (Class|PaperFlipbookComponent|GetFlipbookLength (Variables|Default|GetRenderComponent)) 0.1))
    (CallFunction|RandomMonster)
    (Variables|Default|Sethealth 3.0)
    (Components|Timeline|SetLooping (Variables|Default|GetRenderComponent) true)
    (Sprite|SetFlipbook (Variables|Default|GetRenderComponent) "/Game/Monsters/Monsters_Creatures_Fantasy/Skeleton/skeletonIdle.skeletonIdle")
    (if (== (Variables|Default|GetmonsterType) 0)
      (Sprite|SetFlipbook (Variables|Default|GetRenderComponent) "/Game/Monsters/Monsters_Creatures_Fantasy/Skeleton/skeletonIdle.skeletonIdle")
      (elif (== (Variables|Default|GetmonsterType) 1)
        (Sprite|SetFlipbook (Variables|Default|GetRenderComponent) "/Game/Monsters/Monsters_Creatures_Fantasy/Mushroom/mushroomIdle.mushroomIdle")
        (elif (== (Variables|Default|GetmonsterType) 2)
          (Sprite|SetFlipbook (Variables|Default|GetRenderComponent) "/Game/Monsters/Monsters_Creatures_Fantasy/Goblin/goblinIdle.goblinIdle")
          (elif (== (Variables|Default|GetmonsterType) 3)
            (Sprite|SetFlipbook (Variables|Default|GetRenderComponent) "/Game/Monsters/Monsters_Creatures_Fantasy/Flying_eye/eyeIdle.eyeIdle")))))
    (else
      ;[1 1 1] Mushroom death
      (if (== (Variables|Default|GetmonsterType) 1)
        (Sprite|SetFlipbook (Variables|Default|GetRenderComponent) "/Game/Monsters/Monsters_Creatures_Fantasy/Mushroom/mushroomDeath.mushroomDeath")
        (Components|Timeline|SetLooping (Variables|Default|GetRenderComponent) false)
        (Utilities|FlowControl|Delay (Class|PaperFlipbookComponent|GetFlipbookLength (Variables|Default|GetRenderComponent)))
        (CallFunction|RandomMonster)
        (Variables|Default|Sethealth 3.0)
        (Components|Timeline|SetLooping (Variables|Default|GetRenderComponent) true)
        (Sprite|SetFlipbook (Variables|Default|GetRenderComponent) "/Game/Monsters/Monsters_Creatures_Fantasy/Mushroom/mushroomIdle.mushroomIdle")
        (if (== (Variables|Default|GetmonsterType) 0)
          (Sprite|SetFlipbook (Variables|Default|GetRenderComponent) "/Game/Monsters/Monsters_Creatures_Fantasy/Skeleton/skeletonIdle.skeletonIdle")
          (elif (== (Variables|Default|GetmonsterType) 1)
            (Sprite|SetFlipbook (Variables|Default|GetRenderComponent) "/Game/Monsters/Monsters_Creatures_Fantasy/Mushroom/mushroomIdle.mushroomIdle")
            (elif (== (Variables|Default|GetmonsterType) 2)
              (Sprite|SetFlipbook (Variables|Default|GetRenderComponent) "/Game/Monsters/Monsters_Creatures_Fantasy/Goblin/goblinIdle.goblinIdle")
              (elif (== (Variables|Default|GetmonsterType) 3)
                (Sprite|SetFlipbook (Variables|Default|GetRenderComponent) "/Game/Monsters/Monsters_Creatures_Fantasy/Flying_eye/eyeIdle.eyeIdle")))))
        (else
          ;[1 1 1] Goblin death
          (if (== (Variables|Default|GetmonsterType) 2)
            (Sprite|SetFlipbook (Variables|Default|GetRenderComponent) "/Game/Monsters/Monsters_Creatures_Fantasy/Goblin/goblinDeath.goblinDeath")
            (Components|Timeline|SetLooping (Variables|Default|GetRenderComponent) false)
            (Utilities|FlowControl|Delay (Class|PaperFlipbookComponent|GetFlipbookLength (Variables|Default|GetRenderComponent)))
            (CallFunction|RandomMonster)
            (Variables|Default|Sethealth 3.0)
            (Components|Timeline|SetLooping (Variables|Default|GetRenderComponent) true)
            (Sprite|SetFlipbook (Variables|Default|GetRenderComponent) "/Game/Monsters/Monsters_Creatures_Fantasy/Goblin/goblinIdle.goblinIdle")
            (if (== (Variables|Default|GetmonsterType) 0)
              (Sprite|SetFlipbook (Variables|Default|GetRenderComponent) "/Game/Monsters/Monsters_Creatures_Fantasy/Skeleton/skeletonIdle.skeletonIdle")
              (elif (== (Variables|Default|GetmonsterType) 1)
                (Sprite|SetFlipbook (Variables|Default|GetRenderComponent) "/Game/Monsters/Monsters_Creatures_Fantasy/Mushroom/mushroomIdle.mushroomIdle")
                (elif (== (Variables|Default|GetmonsterType) 2)
                  (Sprite|SetFlipbook (Variables|Default|GetRenderComponent) "/Game/Monsters/Monsters_Creatures_Fantasy/Goblin/goblinIdle.goblinIdle")
                  (elif (== (Variables|Default|GetmonsterType) 3)
                    (Sprite|SetFlipbook (Variables|Default|GetRenderComponent) "/Game/Monsters/Monsters_Creatures_Fantasy/Flying_eye/eyeIdle.eyeIdle")))))
            (else
              ;[1 1 1] Eye death
              (if (== (Variables|Default|GetmonsterType) 3)
                (Sprite|SetFlipbook (Variables|Default|GetRenderComponent) "/Game/Monsters/Monsters_Creatures_Fantasy/Flying_eye/eyeDeath.eyeDeath")
                (Components|Timeline|SetLooping (Variables|Default|GetRenderComponent) false)
                (Utilities|FlowControl|Delay (- (Class|PaperFlipbookComponent|GetFlipbookLength (Variables|Default|GetRenderComponent)) 0.2))
                (CallFunction|RandomMonster)
                (Variables|Default|Sethealth 3.0)
                (Components|Timeline|SetLooping (Variables|Default|GetRenderComponent) true)
                (Sprite|SetFlipbook (Variables|Default|GetRenderComponent) "/Game/Monsters/Monsters_Creatures_Fantasy/Flying_eye/eyeIdle.eyeIdle")
                (if (== (Variables|Default|GetmonsterType) 0)
                  (Sprite|SetFlipbook (Variables|Default|GetRenderComponent) "/Game/Monsters/Monsters_Creatures_Fantasy/Skeleton/skeletonIdle.skeletonIdle")
                  (elif (== (Variables|Default|GetmonsterType) 1)
                    (Sprite|SetFlipbook (Variables|Default|GetRenderComponent) "/Game/Monsters/Monsters_Creatures_Fantasy/Mushroom/mushroomIdle.mushroomIdle")
                    (elif (== (Variables|Default|GetmonsterType) 2)
                      (Sprite|SetFlipbook (Variables|Default|GetRenderComponent) "/Game/Monsters/Monsters_Creatures_Fantasy/Goblin/goblinIdle.goblinIdle")
                      (elif (== (Variables|Default|GetmonsterType) 3)
                        (Sprite|SetFlipbook (Variables|Default|GetRenderComponent) "/Game/Monsters/Monsters_Creatures_Fantasy/Flying_eye/eyeIdle.eyeIdle")))))))))))))

(event Custom|doDamage
  (if (== (Variables|Default|GetmonsterType) 0)
    ;[1 1 1] Skeleton hit
    (if (> (Variables|Default|Gethealth) 0)
      (Variables|Default|Sethealth (- (Variables|Default|Gethealth) 1))
      (CallFunction|UpdateHP)
      (Sprite|SetFlipbook (Variables|Default|GetRenderComponent) "/Game/Monsters/Monsters_Creatures_Fantasy/Skeleton/skeletonIdle.skeletonIdle")
      (Sprite|SetFlipbook (Variables|Default|GetRenderComponent) "/Game/Monsters/Monsters_Creatures_Fantasy/Skeleton/skeletonHit.skeletonHit")
      (Components|Timeline|SetLooping (Variables|Default|GetRenderComponent) false)
      (Utilities|FlowControl|Delay (Class|PaperFlipbookComponent|GetFlipbookLength (Variables|Default|GetRenderComponent)))
      (Sprite|SetFlipbook (Variables|Default|GetRenderComponent) "/Game/Monsters/Monsters_Creatures_Fantasy/Skeleton/skeletonIdle.skeletonIdle")
      (Components|Timeline|SetLooping (Variables|Default|GetRenderComponent) true))
    (else
      ;[1 1 1] Mushroom hit
      (if (== (Variables|Default|GetmonsterType) 1)
        (if (> (Variables|Default|Gethealth) 0)
          (Variables|Default|Sethealth (- (Variables|Default|Gethealth) 1))
          (Sprite|SetFlipbook (Variables|Default|GetRenderComponent) "/Game/Monsters/Monsters_Creatures_Fantasy/Mushroom/mushroomIdle.mushroomIdle")
          (Sprite|SetFlipbook (Variables|Default|GetRenderComponent) "/Game/Monsters/Monsters_Creatures_Fantasy/Mushroom/mushroomHit.mushroomHit")
          (Components|Timeline|SetLooping (Variables|Default|GetRenderComponent) false)
          (Utilities|FlowControl|Delay (Class|PaperFlipbookComponent|GetFlipbookLength (Variables|Default|GetRenderComponent)))
          (Sprite|SetFlipbook (Variables|Default|GetRenderComponent) "/Game/Monsters/Monsters_Creatures_Fantasy/Mushroom/mushroomIdle.mushroomIdle")
          (Components|Timeline|SetLooping (Variables|Default|GetRenderComponent) true))
        (else
          ;[1 1 1] Goblin hit
          (if (== (Variables|Default|GetmonsterType) 2)
            (if (> (Variables|Default|Gethealth) 0)
              (Variables|Default|Sethealth (- (Variables|Default|Gethealth) 1))
              (Sprite|SetFlipbook (Variables|Default|GetRenderComponent) "/Game/Monsters/Monsters_Creatures_Fantasy/Goblin/goblinIdle.goblinIdle")
              (Sprite|SetFlipbook (Variables|Default|GetRenderComponent) "/Game/Monsters/Monsters_Creatures_Fantasy/Goblin/goblinHit.goblinHit")
              (Components|Timeline|SetLooping (Variables|Default|GetRenderComponent) false)
              (Utilities|FlowControl|Delay (Class|PaperFlipbookComponent|GetFlipbookLength (Variables|Default|GetRenderComponent)))
              (Sprite|SetFlipbook (Variables|Default|GetRenderComponent) "/Game/Monsters/Monsters_Creatures_Fantasy/Goblin/goblinIdle.goblinIdle")
              (Components|Timeline|SetLooping (Variables|Default|GetRenderComponent) true))
            (else
              ;[1 1 1] Eye hit
              (if (== (Variables|Default|GetmonsterType) 3)
                (if (> (Variables|Default|Gethealth) 0)
                  (Variables|Default|Sethealth (- (Variables|Default|Gethealth) 1))
                  (Sprite|SetFlipbook (Variables|Default|GetRenderComponent) "/Game/Monsters/Monsters_Creatures_Fantasy/Flying_eye/eyeIdle.eyeIdle")
                  (Sprite|SetFlipbook (Variables|Default|GetRenderComponent) "/Game/Monsters/Monsters_Creatures_Fantasy/Flying_eye/eyeHit.eyeHit")
                  (Components|Timeline|SetLooping (Variables|Default|GetRenderComponent) false)
                  (Utilities|FlowControl|Delay (Class|PaperFlipbookComponent|GetFlipbookLength (Variables|Default|GetRenderComponent)))
                  (Sprite|SetFlipbook (Variables|Default|GetRenderComponent) "/Game/Monsters/Monsters_Creatures_Fantasy/Flying_eye/eyeIdle.eyeIdle")
                  (Components|Timeline|SetLooping (Variables|Default|GetRenderComponent) true))))))))))

(event Custom|playTimer
  (bind _returnvalue (AddComponent|AddAudioComponent false))
  (Variables|Default|Setaudio _returnvalue))

(event Custom|stopTimer
  (if (<= (Variables|Default|GetplayerLives) 0)
    (Audio|Components|Audio|Stop (Variables|Default|Getaudio))))

(event EventBeginPlay
  (CallFunction|UpdateHP)
  (Sprite|SetFlipbook (Variables|Default|GetRenderComponent) "/Game/Monsters/Monsters_Creatures_Fantasy/Skeleton/skeletonIdle.skeletonIdle")
  (CallFunction|PlayTimer)
  (Variables|/Script/Engine.PlayerController|SetbEnableClickEvents (Game|GetPlayerController 0) true)
  ;[1 1 1] Set Skeleton
  (if (== (Variables|Default|GetmonsterType) 0)
    (Sprite|SetFlipbook (Variables|Default|GetRenderComponent) "/Game/Monsters/Monsters_Creatures_Fantasy/Skeleton/skeletonIdle.skeletonIdle")
    (else
      ;[1 1 1] Set Mushroom
      (if (== (Variables|Default|GetmonsterType) 1)
        (Sprite|SetFlipbook (Variables|Default|GetRenderComponent) "/Game/Monsters/Monsters_Creatures_Fantasy/Mushroom/mushroomIdle.mushroomIdle")
        (else
          ;[1 1 1] Set Goblin
          (if (== (Variables|Default|GetmonsterType) 2)
            (Sprite|SetFlipbook (Variables|Default|GetRenderComponent) "/Game/Monsters/Monsters_Creatures_Fantasy/Goblin/goblinIdle.goblinIdle")
            (else
              ;[1 1 1] Set Goblin
              (if (== (Variables|Default|GetmonsterType) 3)
                (Sprite|SetFlipbook (Variables|Default|GetRenderComponent) "/Game/Monsters/Monsters_Creatures_Fantasy/Flying_eye/eyeIdle.eyeIdle")))))))))

(event EventTick
  (params (DeltaSeconds :type Float%20%28single-precision%29))
  (if (<= (Variables|Default|GetplayerLives) 0)
    (Class|AchievementSubSystem|AddAchievementProgress (Subsystems|GetAchievementSubSystem) "Ach3" 1.0)
    (CallFunction|UpdateHP)
    (CallFunction|CheckPlayerLives)
    (CallFunction|StopTimer)
    (if (<= (Variables|Default|Gethealth) 0)
      (CallFunction|Death)
      (bind _ashealth_widget (Utilities|Casting|CastToHealthWidget (UserInterface|GetUserWidgetObject (Variables|Default|GetHPBar))))
      (Variables|/Game/Blueprints/HealthBarShit/HealthWidget.HealthWidget_C|SetWidgetHealth _ashealth_widget (Variables|Default|Gethealth)))))

(fn ConstructionScript)

(fn UpdateHP
  (bind _ashealth_widget (Utilities|Casting|CastToHealthWidget (UserInterface|GetUserWidgetObject (Variables|Default|GetHPBar))))
  (Variables|/Game/Blueprints/HealthBarShit/HealthWidget.HealthWidget_C|SetWidgetHealth _ashealth_widget (Variables|Default|Gethealth))
  (return))