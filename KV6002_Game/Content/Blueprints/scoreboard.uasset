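; Scoreboard Blueprint that reads saved time and score entries from the DT_TimerStats data table, with only debug printing as output.
; Its getTimerStats event picks a random row and copies its Time and Score into Time1 and ScoreGrab, then prints a placeholder message.
; The stored values print only when the row lookup fails, and nothing in this Blueprint calls the event.
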(event Custom|getTimerStats
  (bind _outrownames (DataTable|GetDataTableRowNames "/Game/DataTables/DT_TimerStats.DT_TimerStats"))
  (bind _returnvalue (Utilities|GetDataTableRow "/Game/DataTables/DT_TimerStats.DT_TimerStats" (Utilities|Array|Get(acopy) _outrownames (Math|Random|RandomInteger (Utilities|Array|Length _outrownames))))
    (:then
      (bind _output_get (Variables|Default|SetTime1 (.Time (Utilities|Struct|BreakS_TimerStats _returnvalue))))
      (bind _output_get_2 (Variables|Default|SetscoreGrab (.score (Utilities|Struct|BreakS_TimerStats _returnvalue))))
      (Development|PrintString "Hello"))
    (:RowNotFound
      (Development|PrintString _output_get)
      (Development|PrintString (Utilities|String|ToString(Integer) _output_get_2)))))

(event EventBeginPlay)

(event EventTick
  (params (DeltaSeconds :type Float%20%28single-precision%29)))

(fn ConstructionScript)