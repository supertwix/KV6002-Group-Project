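; Login actor that authenticates the player against a web token endpoint from the LoginUI widget.
; On submit, it sends the username and password as a Base64 Basic-style Authorization header via VaRest.
; It string-splits the token from the response and verifies it with EasyJwt using a hard-coded HS256 key.
; Success stores the "sub" claim as Id and opens the main menu after a Leaderboard cast, while failed verification shows the incorrect-login message.
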(event Custom|SubmitButtonClicked
  (bind _returnvalue (|EasyJwtSubsystem))
  (Development|PrintString "submit button clicked")
  (bind _output_get (Variables|Default|SetUsername (Utilities|String|ToString(Text) (Class|EditableText|GetText (Variables|/Game/Blueprints/LoginUI.LoginUI_C|GetUsernameInput (Utilities|Array|Get(acopy) (stale EventBeginPlay _foundwidgets)))))))
  (bind _output_get_2 (Variables|Default|SetPassword (Utilities|String|ToString(Text) (Class|EditableText|GetText (Variables|/Game/Blueprints/LoginUI.LoginUI_C|GetPasswordInput (Utilities|Array|Get(acopy) (stale EventBeginPlay _foundwidgets)))))))
  (bind _output_get_3 (Variables|Default|SetHeader%20Value (Utilities|String|Append (Utilities|String|MakeLiteralString "Basic : ") (Utilities|String|MakeLiteralString (Class|VaRestLibrary|Base64Encode (Utilities|String|Append (Utilities|String|Append _output_get ":") _output_get_2))))))
  (bind _returnvalue_2 (Class|VaRestSubsystem|ConstructVaRestRequestExt (|VaRestSubsystem) "GET" "x_www_form_urlencoded_body"))
  (bind _output_get_4 (Variables|Default|SetRequestHeader _returnvalue_2))
  (Class|VaRestRequestJSON|SetHeader _output_get_4 "Authorization" _output_get_3)
  (bind _result (Class|VaRestRequestJSON|ApplyURL _output_get_4 "https://w20013126.nuwebspace.co.uk/GroupProjectSem2/token"))
  (Class|EasyJwtSubsystem|InitVerifier _returnvalue "Tr9FA1lOAtEbmUbfsms91EXpyBglsPRJ" "HS256")
  (bind _returnvalue_3 (Class|EasyJwtSubsystem|VerifyJWT _returnvalue (.LeftS (Utilities|String|Split (.RightS (Utilities|String|Split (.RightS (Utilities|String|Split (Class|VaRestJsonObject|EncodeJson _result) ":")) "\"")) "\""))))
  (if _returnvalue_3
    (bind _returnvalue_4 (Class|EasyJwtSubsystem|GetClaims _returnvalue (.LeftS (Utilities|String|Split (.RightS (Utilities|String|Split (.RightS (Utilities|String|Split (Class|VaRestJsonObject|EncodeJson _result) ":")) "\"")) "\""))))
    (Development|PrintString (.Value (Utilities|Map|Find _returnvalue_4 "sub")))
    (Variables|Default|Setid (.Value (Utilities|Map|Find _returnvalue_4 "sub")))
    (Utilities|Casting|CastToWidgetClass "/Game/Blueprints/MenuAndHUD/Leaderboard.Leaderboard_C")
    (Development|PrintString "worked :)")
    (Game|OpenLevel(byName) "MainMenuLv")
    (else
      (Development|PrintString "not worked lol")
      (Widget|SetVisibility (Variables|/Game/Blueprints/LoginUI.LoginUI_C|GetIncorrectLogin (Utilities|Array|Get(acopy) (stale EventBeginPlay _foundwidgets))) "Visible"))))

(event EventBeginPlay
  (bind _foundwidgets (Widget|GetAllWidgetsOfClass "/Game/Blueprints/LoginUI.LoginUI_C" false))
  (Widget|SetVisibility (Variables|/Game/Blueprints/LoginUI.LoginUI_C|GetIncorrectLogin (Utilities|Array|Get(acopy) _foundwidgets)) "Hidden")
  (EventDispatchers|BindEventtoOnClicked (Variables|/Game/Blueprints/LoginUI.LoginUI_C|GetSubmitButton (Utilities|Array|Get(acopy) _foundwidgets)) (delegate Custom|SubmitButtonClicked)))

(fn ConstructionScript)