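; GetQuestion is a quiz helper Blueprint that picks a random question from the Questions data table.
; It copies the row's question, correct answer and three wrong answers into its own variables, printing a message if the row is missing.
; This runs on BeginPlay and again whenever the getQuestions event is called, using duplicated logic with no guard against repeats.
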(event Custom|getQuestions
  (bind _outrownames (DataTable|GetDataTableRowNames "/Game/DataTables/Questions.Questions"))
  (bind _returnvalue (Utilities|GetDataTableRow "/Game/DataTables/Questions.Questions" (Utilities|Array|Get(acopy) _outrownames (Math|Random|RandomInteger (Utilities|Array|Length _outrownames))))
    (:then
      (Variables|Default|Setquestion (.Question (Utilities|Struct|BreakSQuestionGen _returnvalue)))
      (Variables|Default|Setanswer (.Answer (Utilities|Struct|BreakSQuestionGen _returnvalue)))
      (Variables|Default|Setwrong1 (.WrongAnswer1 (Utilities|Struct|BreakSQuestionGen _returnvalue)))
      (Variables|Default|Setwrong2 (.WrongAnswer2 (Utilities|Struct|BreakSQuestionGen _returnvalue)))
      (Variables|Default|Setwrong3 (.WrongAnswer3 (Utilities|Struct|BreakSQuestionGen _returnvalue))))
    (:RowNotFound
      (Development|PrintString "row not found"))))

(event EventBeginPlay
  (bind _outrownames (DataTable|GetDataTableRowNames "/Game/DataTables/Questions.Questions"))
  (bind _returnvalue (Utilities|GetDataTableRow "/Game/DataTables/Questions.Questions" (Utilities|Array|Get(acopy) _outrownames (Math|Random|RandomInteger (Utilities|Array|Length _outrownames))))
    (:then
      (Variables|Default|Setquestion (.Question (Utilities|Struct|BreakSQuestionGen _returnvalue)))
      (Variables|Default|Setanswer (.Answer (Utilities|Struct|BreakSQuestionGen _returnvalue)))
      (Variables|Default|Setwrong1 (.WrongAnswer1 (Utilities|Struct|BreakSQuestionGen _returnvalue)))
      (Variables|Default|Setwrong2 (.WrongAnswer2 (Utilities|Struct|BreakSQuestionGen _returnvalue)))
      (Variables|Default|Setwrong3 (.WrongAnswer3 (Utilities|Struct|BreakSQuestionGen _returnvalue))))
    (:RowNotFound
      (Development|PrintString "row not found"))))

(fn ConstructionScript)