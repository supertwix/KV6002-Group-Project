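; CyberTimer is a Blueprint that keeps an elapsed-time count in minutes and seconds and puts a timer widget on screen.
; BeginPlay creates the Timer widget and adds it to the viewport.
; Tick runs through a one-second Delay, which throttles the count to roughly once per second, then increments Seconds and rolls it over into Minutes after 59.
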(event EventBeginPlay
  ;[1 1 1] Allows the timer to be visable to the user.
  (bind _returnvalue (UserInterface|CreateWidget "/Game/Blueprints/Timer.Timer_C"))
  (UserInterface|Viewport|AddtoViewport _returnvalue 0))

(event EventTick
  (params (DeltaSeconds :type Float%20%28single-precision%29))
  ;[1 1 1] The creation of the functionality of Cybertimer.
  (Utilities|FlowControl|Delay 1.0)
  (Variables|Default|SetSeconds (+ (Variables|Default|GetSeconds) 1))
  (if (> (Variables|Default|GetSeconds) 59)
    (Variables|Default|SetMinutes (+ (Variables|Default|GetMinutes) 1))
    (Variables|Default|SetSeconds 0)))

(fn ConstructionScript)